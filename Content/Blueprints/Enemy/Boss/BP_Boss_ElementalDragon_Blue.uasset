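; Blue elemental dragon boss Blueprint that implements a tornado attack through the SpawnTornado event.
; A timeline nudges the dragon backward along its facing with a swept move on each update.
; The same update feeds a one-second Delay, which throttles volleys of three ProjectileClass actors: a large central one and two smaller, lower ones angled to either side.
; A LaunchCharacter call is left unconnected.
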(event EventSpawnTornado
  (bind _returnvalue (Transformation|GetActorForwardVector))
  (bind _returnvalue_2 (Transformation|GetActorLocation))
  (bind _returnvalue_3 (Transformation|GetActorLocation))
  (bind _returnvalue_4 (Transformation|GetActorForwardVector))
  (bind _returnvalue_5 (Transformation|GetActorLocation))
  (bind _returnvalue_6 (Transformation|GetActorLocation))
  (bind _returnvalue_7 (Math|Conversions|RotationFromXVector _returnvalue))
  (bind _returnvalue_8 (Math|Conversions|RotationFromXVector _returnvalue_4))
  (bind _newtrack_1 (Timeline|Timeline PlayFromStart)
    (:Update
      (Transformation|SetActorLocation (Math|Vector|Lerp(Vector) _returnvalue_3 (+ _returnvalue_3 (* (Transformation|GetActorForwardVector) -5e+01)) _newtrack_1) true false)
      (Utilities|FlowControl|Delay 1.0)
      (Game|SpawnActorfromClass (Variables|Default|GetProjectileClass) (Math|Transform|MakeTransform (Math|Vector|MakeVector (.x _returnvalue_2) (.y _returnvalue_2) (+ (.z _returnvalue_2) 8e+02)) (Math|Conversions|RotationFromXVector (Transformation|GetActorForwardVector)) "15.000000,15.000000,15.000000") "Undefined" "MultiplyWithRoot" 0 0)
      (Game|SpawnActorfromClass (Variables|Default|GetProjectileClass) (Math|Transform|MakeTransform (Math|Vector|MakeVector (.x _returnvalue_5) (.y _returnvalue_5) (+ (.z _returnvalue_5) 5e+02)) (Math|Rotator|MakeRotator (.roll _returnvalue_8) (.pitch _returnvalue_8) (+ (.yaw _returnvalue_8) 25.0)) "10.000000,10.000000,10.000000") "Undefined" "MultiplyWithRoot" 0 0)
      (Game|SpawnActorfromClass (Variables|Default|GetProjectileClass) (Math|Transform|MakeTransform (Math|Vector|MakeVector (.x _returnvalue_6) (.y _returnvalue_6) (+ (.z _returnvalue_6) 5e+02)) (Math|Rotator|MakeRotator (.roll _returnvalue_7) (.pitch _returnvalue_7) (+ (.yaw _returnvalue_7) -25.0)) "10.000000,10.000000,10.000000") "Undefined" "MultiplyWithRoot" 0 0))))

(fn ConstructionScript)