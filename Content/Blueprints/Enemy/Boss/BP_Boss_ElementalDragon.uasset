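; Elemental dragon boss Blueprint with an encounter intro and a tornado attack, both switching the character between flying and walking.
; BossEncounter sets an AI blackboard flag, plays a montage, and uses a timeline angle to orbit high above its starting point.
; SpawnTornado uses a timeline to lift the dragon backward, then spawns three oversized projectiles in a forward fan.
; Delays hanging off timeline updates time the projectile spawns and walking switches.
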(event EventSpawnTornado
  (bind _returnvalue (Transformation|GetActorForwardVector))
  (bind _returnvalue_2 (Transformation|GetActorLocation))
  (bind _returnvalue_3 (Transformation|GetActorLocation))
  (bind _returnvalue_4 (Transformation|GetActorForwardVector))
  (bind _returnvalue_5 (Transformation|GetActorLocation))
  (bind _returnvalue_6 (Transformation|GetActorLocation))
  (bind _returnvalue_7 (Math|Conversions|RotationFromXVector _returnvalue))
  (bind _returnvalue_8 (Math|Conversions|RotationFromXVector _returnvalue_4))
  (Pawn|Components|CharacterMovement|SetMovementMode (Variables|Character|GetCharacterMovement) "MOVE_Flying" 0)
  (bind _newtrack_1 (Timeline|Timeline_Tornado PlayFromStart)
    (:Update
      (Transformation|SetActorLocation (Math|Vector|Lerp(Vector) _returnvalue_3 (+ (+ _returnvalue_3 (* (Transformation|GetActorForwardVector) -5e+01)) "0.000000,0.000000,20.000000") _newtrack_1) true false)
      (Utilities|FlowControl|Delay 1.0)
      (Game|SpawnActorfromClass (Variables|Default|GetProjectileClass) (Math|Transform|MakeTransform (Math|Vector|MakeVector (.x _returnvalue_2) (.y _returnvalue_2) (+ (.z _returnvalue_2) 3e+02)) (Math|Conversions|RotationFromXVector (Transformation|GetActorForwardVector)) "15.000000,15.000000,15.000000") "Undefined" "MultiplyWithRoot" 0 0)
      (Game|SpawnActorfromClass (Variables|Default|GetProjectileClass) (Math|Transform|MakeTransform (Math|Vector|MakeVector (.x _returnvalue_5) (.y _returnvalue_5) (+ (.z _returnvalue_5) 3e+02)) (Math|Rotator|MakeRotator (.roll _returnvalue_8) (.pitch _returnvalue_8) (+ (.yaw _returnvalue_8) 25.0)) "15.000000,15.000000,15.000000") "Undefined" "MultiplyWithRoot" 0 0)
      (Game|SpawnActorfromClass (Variables|Default|GetProjectileClass) (Math|Transform|MakeTransform (Math|Vector|MakeVector (.x _returnvalue_6) (.y _returnvalue_6) (+ (.z _returnvalue_6) 3e+02)) (Math|Rotator|MakeRotator (.roll _returnvalue_7) (.pitch _returnvalue_7) (+ (.yaw _returnvalue_7) -25.0)) "15.000000,15.000000,15.000000") "Undefined" "MultiplyWithRoot" 0 0)
      (Pawn|Components|CharacterMovement|SetMovementMode (Variables|Character|GetCharacterMovement) "MOVE_Walking" 0))))

(event EventBossEncounter
  (Variables|Default|SetOrbitCenter (Transformation|GetActorLocation))
  (AI|Components|Blackboard|SetValueasBool (Variables|/Script/AIModule.AIController|GetBlackboard (.AsARAIController (Utilities|Casting|CastToARAIController (AI|GetAIController self)))) (Variables|Default|GetKey%20Name) true)
  (Pawn|Components|CharacterMovement|SetMovementMode (Variables|Character|GetCharacterMovement) "MOVE_Flying" 0)
  (Transformation|Teleport (Variables|Default|GetOrbitCenter) "0.000000,140.000000,0.000000")
  (Animation|Montage|PlayMontage (Variables|Character|GetMesh) "/Game/Animation/Enemy/Boss/Elemental_Dragon/AM_Encounter.AM_Encounter"
    (:then
      (bind _angle (Timeline|Timeline_Encounter Play)
        (:Update
          (Transformation|SetActorLocation (+ (* (Math|Vector|GetForwardVector (Math|Rotator|MakeRotator 0.0 0.0 _angle)) (Variables|Default|GetOrbitRadius)) (+ (Variables|Default|GetOrbitCenter) "0.000000,0.000000,5000.000000")) false false)
          (Utilities|FlowControl|Delay 3.999)
          (Pawn|Components|CharacterMovement|SetMovementMode (Variables|Character|GetCharacterMovement) "MOVE_Walking" 0))))))

(fn ConstructionScript)