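; Test player controller for the quest system that sets up the quest UI when play begins.
; BeginPlay adds BP_QuestTestHUD and a second widget, whose class comes from a variable, to the viewport.
; It then binds the second widget to the QuestComponent tagged "AA" on player pawn 0, if one is found.
; An unconnected branch that would create a third widget never runs.
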(event EventBeginPlay
  (bind _returnvalue (Game|Player|GetPlayerPawn 0))
  (bind _returnvalue_2 (Class|Actor|FindComponentbyTag _returnvalue "/Script/Arua.QuestComponent" "AA"))
  (Utilities|FlowControl|Sequence
    (:then_0
      (bind _returnvalue_3 (UserInterface|CreateWidget "/Game/Personal/KIM_J_H/TestAssets/BP_QuestTestHUD.BP_QuestTestHUD_C" self))
      (UserInterface|Viewport|AddtoViewport _returnvalue_3 0))
    (:then_1
      (bind _returnvalue_4 (UserInterface|CreateWidget (Variables|Default|GetNewVar) self))
      (UserInterface|Viewport|AddtoViewport _returnvalue_4 0))
    (:then_3
      (Utilities|IsValid _returnvalue_2
        (:Is%20Valid
          (Class|QuestHUDWidget|BindtoQuestComponent _returnvalue_4 _returnvalue_2))))))

(event EventTick
  (params (DeltaSeconds :type Float%20%28single-precision%29)))

(fn ConstructionScript)